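; BP_Spikes is a spike hazard that deals physical damage to the player pawn while it overlaps the actor.
; Begin and end overlap share one branch that toggles PokingPlayer and primes HitTime, so the first hit lands immediately.
; Tick accumulates HitTime and applies damage to the overlapping BP_PlayerCharacter roughly once per second.
; BeginPlay caches the GamayHUD reference, which is otherwise unused here.
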(event `self.ReceiveBeginPlay`
  (bind _asui_gamay_hud (cast `/Game/Assets/Blueprints/UI/UI_GamayHUD` (`PlayerController.GetHUD` (`GameplayStatics.GetPlayerController` 0))))
  (set `self.GamayHUD` _asui_gamay_hud))

(event `self.ReceiveActorEndOverlap`
  (params (OtherActor :type "Actor Object Reference"))
  (if (== (stale `self.ReceiveActorBeginOverlap` OtherActor) (`GameplayStatics.GetPlayerPawn` 0)) :!label _label
    (set `self.pokingPlayer` (not (`self.pokingPlayer`)))
    (set `self.hitTime` 1.0)))

(event `self.ReceiveActorBeginOverlap`
  (params (OtherActor :type "Actor Object Reference"))
  (goto _label))

(event `self.ReceiveTick`
  (params (DeltaSeconds :type "Float (single-precision)"))
  (bind _hittime (`self.hitTime`))
  (if (`self.pokingPlayer`)
    (if (and (< (- _hittime DeltaSeconds) 1.0) (>= _hittime 1.0))
      (bind _asbp_player_character (cast `/Game/Assets/Blueprints/Entities/Characters/Humans/BP_PlayerCharacter` (stale `self.ReceiveActorBeginOverlap` OtherActor)))
      (`GameplayStatics.ApplyDamage` _asbp_player_character 25.0 null self "/Game/Assets/Blueprints/DamageTypes/DamageType_Physical.DamageType_Physical_C")
      (set `self.hitTime` 0.0)
      (else
        (bind _output_get (set `self.hitTime` (+ (stale _output_get) DeltaSeconds)))))))

(fn `UserConstructionScript`)