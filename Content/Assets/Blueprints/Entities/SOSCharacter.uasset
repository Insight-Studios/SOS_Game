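; SOSCharacter is a character Blueprint that holds experience and level progression, with no active event graph logic.
; AddXP adds to CurrentXP and, once it reaches NeededXP, raises CurrentLevel, carries the surplus over and calls OnLevelUp.
; Each call grants at most one level and leaves NeededXP unchanged; OnLevelUp is an empty hook.
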(fn `AddXP`
  (params (`Added XP` :type "Float (double-precision)"))
  (bind _neededxp (`self.NeededXP`))
  (bind _output_get (set `self.CurrentXP` (+ `Added XP` (`self.CurrentXP`))))
  (if (>= _output_get _neededxp)
    (`/Engine/EditorBlueprintResources/StandardMacros.IncrementInt` (`self.CurrentLevel`)
      (:`  `
        (set `self.CurrentXP` (- _output_get _neededxp))
        (`self.OnLevelUp`)))))

(fn `OnLevelUp`)

(fn `UserConstructionScript`
  (`parent.UserConstructionScript`))