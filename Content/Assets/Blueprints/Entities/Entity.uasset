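; Base entity Blueprint with health, interaction-range and highlight behavior, plus empty OnDeath and Pickup functions.
; AnyDamage forwards positive values to HealthSystem as damage and routes others to RecieveHeal, though without passing a heal amount.
; InteractableArea overlaps register and unregister the entity's interact message with the PlayerCharacter.
; SetHighlight toggles custom depth rendering on InteractableArea.
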(event `self.ReceiveBeginPlay`)

(event `self.ReceiveAnyDamage`
  (params (Damage :type "Float (single-precision)") (DamageType :type "DamageType Object Reference") (InstigatedBy :type "Controller Object Reference") (DamageCauser :type "Actor Object Reference"))
  (bind _asdamage_type (castclass `DamageType` (`GameplayStatics.GetObjectClass` DamageType)))
  (if (> Damage 0.0)
    (`self.Recieve Damage` Damage InstigatedBy DamageCauser _asdamage_type)
    (else
      (`self.Recieve Heal` 0.0 null null _asdamage_type))))

(event `self.InteractableArea.OnComponentBeginOverlap`
  (params (OverlappedComponent :type "PrimitiveComponent Object Reference") (OtherActor :type "Actor Object Reference") (OtherComp :type "PrimitiveComponent Object Reference") (OtherBodyIndex :type Integer) (bFromSweep :type Boolean) (SweepResult :type "HitResult Structure (by ref)"))
  (bind _asplayer_character (cast `/Game/Assets/Blueprints/Entities/PlayerCharacter` OtherActor))
  (message `/Game/Assets/Blueprints/Entities/BPI_Interact.RegisterInteractable` _asplayer_character self))

(event `self.InteractableArea.OnComponentEndOverlap`
  (params (OverlappedComponent :type "PrimitiveComponent Object Reference") (OtherActor :type "Actor Object Reference") (OtherComp :type "PrimitiveComponent Object Reference") (OtherBodyIndex :type Integer))
  (bind _asplayer_character (cast `/Game/Assets/Blueprints/Entities/PlayerCharacter` OtherActor))
  (message `/Game/Assets/Blueprints/Entities/BPI_Interact.UnregisterInteractable` _asplayer_character self))

(fn `On Death`)

(fn `Pickup`
  (params (ItemInfo :type "/Game/Assets/Blueprints/Entities/Items/ItemInfo Structure")))

(fn `Recieve Damage`
  (params (`Base Damage` :type "Float (double-precision)") (`Instigated By` :type "Controller Object Reference") (`Damage Causer` :type "Actor Object Reference") (`Damage Type Class` :type "DamageType Class Reference"))
  (`/Game/Assets/Blueprints/ModularSystems/healthSystem.applyDamage` (`self.HealthSystem`) `Base Damage`))

(fn `Recieve Heal`
  (params (`Base Heal` :type "Float (double-precision)") (`Event Instigator` :type "Controller Object Reference") (`Heal Causer` :type "Actor Object Reference") (`Damage Type Class` :type "DamageType Class Reference"))
  (`/Game/Assets/Blueprints/ModularSystems/healthSystem.applyHeal` (`self.HealthSystem`) `Base Heal`))

(fn `SetHighlight`
  (params (`Highlight?` :type Boolean))
  (`PrimitiveComponent.SetRenderCustomDepth` (`self.InteractableArea`) `Highlight?`))

(fn `UserConstructionScript`)