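; BP_SOSCharacter is a character Blueprint providing health, XP leveling, a capped inventory and equipment slots.
; AnyDamage routes positive amounts to HealthSystem as damage and others to ReceiveHeal, which currently applies zero healing.
; EquipItem spawns item actors on mesh sockets named after the slot enum, tracking them in per-slot maps for replacement and removal.
; OnDeath destroys the actor, while OnLevelUp and UseItem are stubs.
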(event `self.ReceiveAnyDamage`
  (params (Damage :type "Float (single-precision)") (DamageType :type "DamageType Object Reference") (InstigatedBy :type "Controller Object Reference") (DamageCauser :type "Actor Object Reference"))
  (bind _asdamage_type (castclass `DamageType` (`GameplayStatics.GetObjectClass` DamageType)))
  (if (> Damage 0.0)
    (`self.ReceiveDamage` Damage InstigatedBy DamageCauser _asdamage_type)
    (else
      (`self.ReceiveHeal` Damage InstigatedBy DamageCauser _asdamage_type))))

(fn `AddXP`
  (params (`Added XP` :type "Float (double-precision)"))
  (bind _neededxp (`self.NeededXP`))
  (bind _output_get (set `self.CurrentXP` (+ `Added XP` (`self.CurrentXP`))))
  (if (>= _output_get _neededxp)
    (`/Engine/EditorBlueprintResources/StandardMacros.IncrementInt` (`self.CurrentLevel`)
      (:`  `
        (set `self.CurrentXP` (- _output_get _neededxp))
        (`self.OnLevelUp`)))))

(fn `EquipItem`
  (params (ItemSlot :type "/Game/Assets/Blueprints/Entities/Items/ESlotType Enum" :default "NewEnumerator0") (Item :type "/Game/Assets/Blueprints/Entities/Items/FItemInfo Structure"))
  (returns (Equiped :type Boolean))
  (if (`.ReturnValue` (`BlueprintMapLibrary.Map_Find` (`self.EquipedItems`) ItemSlot))
    (`self.UnEquipItem` ItemSlot))
  (bind _returnvalue (`|SpawnActorFromClass` (`.ItemClass_14_94E0F5D144E5BC164CCC3BBDC6AE683E` (break `/Game/Assets/Blueprints/Entities/Items/FItemInfo` Item)) (`self.GetTransform`) "AlwaysSpawn" "OverrideRootScale" null null))
  (`self.SetActorEnableCollision` _returnvalue false)
  (`self.K2_AttachToComponent` _returnvalue (`self.Mesh`) (`KismetStringLibrary.Conv_StringToName` (`|GetEnumeratorNameAsString` ItemSlot)) "SnapToTarget" "SnapToTarget" "SnapToTarget" true)
  (`BlueprintMapLibrary.Map_Add` (`self.EquipedObjects`) ItemSlot _returnvalue)
  (`BlueprintMapLibrary.Map_Add` (`self.EquipedItems`) ItemSlot Item)
  (return true))

(fn `OnDeath`
  (`self.K2_DestroyActor`))

(fn `OnLevelUp`)

(fn `Pickup`
  (params (ItemInfo :type "/Game/Assets/Blueprints/Entities/Items/FItemInfo Structure"))
  (returns (PickedUp :type Boolean))
  (bind _inventory (`self.Inventory`))
  (if (< (`KismetArrayLibrary.Array_Length` _inventory) (`self.InventorySize`))
    (`KismetArrayLibrary.Array_Add` _inventory ItemInfo)
    (return true)
    (else
      (return false))))

(fn `ReceiveDamage`
  (params (`Base Damage` :type "Float (double-precision)") (`Instigated By` :type "Controller Object Reference") (`Damage Causer` :type "Actor Object Reference") (`Damage Type Class` :type "DamageType Class Reference"))
  (`/Game/Assets/Blueprints/ModularSystems/BPC_HealthSystem.applyDamage` (`self.HealthSystem`) `Base Damage`))

(fn `ReceiveHeal`
  (params (`Base Heal` :type "Float (double-precision)") (`Instigated By` :type "Controller Object Reference") (`Heal Cause` :type "Actor Object Reference") (`Damage Type Class` :type "DamageType Class Reference"))
  (`/Game/Assets/Blueprints/ModularSystems/BPC_HealthSystem.applyHeal` (`self.HealthSystem`) 0.0))

(fn `UnEquipItem`
  (params (Slot :type "/Game/Assets/Blueprints/Entities/Items/ESlotType Enum" :default "NewEnumerator0"))
  (returns (Unequiped :type Boolean))
  (bind _equipedobjects (`self.EquipedObjects`))
  (bind (_value _returnvalue) (`BlueprintMapLibrary.Map_Find` _equipedobjects Slot))
  (bind _returnvalue_2 (`BlueprintMapLibrary.Map_Remove` (`self.EquipedItems`) Slot))
  (`self.K2_DestroyActor` _value)
  (bind _returnvalue_3 (`BlueprintMapLibrary.Map_Remove` _equipedobjects Slot))
  (return (and _returnvalue_3 _returnvalue_2 _returnvalue)))

(fn `UseItem`
  (params (ItemInfo :type "/Game/Assets/Blueprints/Entities/Items/FItemInfo Structure"))
  (returns (Used :type Boolean))
  (return false))

(fn `UserConstructionScript`
  (`parent.UserConstructionScript`))