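; BP_BaseItem is a base item actor that characters can pick up through an Interaction event.
; Interaction passes its ItemInfo struct to the character's Pickup function, destroying the actor on success and printing "Oof" on failure.
; The construction script rebuilds ItemInfo with the actor's own class, keeping the other fields, so the struct records which class it came from.
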(event `/Game/Assets/Blueprints/Entities/BPI_Interact.Interaction`
  (params (`Character Reference` :type "/Game/Assets/Blueprints/Entities/Characters/Humans/BP_PlayerCharacter Object Reference"))
  (bind _pickedup (`/Game/Assets/Blueprints/Entities/Characters/BP_SOSCharacter.Pickup` `Character Reference` (`self.ItemInfo`)))
  (if _pickedup
    (`self.K2_DestroyActor`)
    (else
      (`KismetSystemLibrary.PrintString` "Oof"))))

(fn `UserConstructionScript`
  (bind (_iteminfo_itemtype _iteminfo_itemname _iteminfo_itemid _iteminfo_itemclass _iteminfo_itemslots _iteminfo_itemvalue) (break `/Game/Assets/Blueprints/Entities/Items/S_ItemInfo` (`self.ItemInfo`)))
  (`parent.UserConstructionScript`)
  (set `self.ItemInfo` (make `/Game/Assets/Blueprints/Entities/Items/S_ItemInfo` _iteminfo_itemtype _iteminfo_itemname _iteminfo_itemid (`GameplayStatics.GetObjectClass` self) _iteminfo_itemslots _iteminfo_itemvalue)))