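; Modular health component that tracks damage, healing, out-of-combat regeneration and death for its owning actor.
; BeginPlay messages the owner for setup, and Tick regenerates health, updates the health percentage and messages the owner's death handler while health is depleted.
; A per-second macro using near-whole game time advances and prints the combat timer, which damage resets.
; Regeneration accumulates fractions into whole health points once that timer passes its timeout.
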(event `self.ReceiveBeginPlay`
  (message `/Game/Assets/Blueprints/Entity.setupHealthSystem` (`self.GetOwner`)))

(event `self.ReceiveTick`
  (params (DeltaSeconds :type "Float (single-precision)"))
  (`|ExecutionSequence`
    (:`then_0`
      (`self.updateHealth` DeltaSeconds)
      (`self.perSecond` DeltaSeconds
        (:`PerSecond`
          (bind _result (`/Engine/EditorBlueprintResources/StandardMacros.IncrementInt` (`self.combatTimer`))
            (:`  `
              (`KismetSystemLibrary.PrintString` (`KismetStringLibrary.Conv_IntToString` _result)))))))
    (:`then_1`
      (set `self.percentHealth` (/ (`KismetMathLibrary.Conv_IntToDouble` (`self.currentHealth`)) (`KismetMathLibrary.Conv_IntToDouble` (`self.maxHealth`)))))
    (:`then_2`
      (if (<= (`self.currentHealth`) 0)
        (message `/Game/Assets/Blueprints/Entity.onDeath` (`self.GetOwner`))))))

(fn `damageActor`
  (params (amount :type Integer) (`Damage Type` :type "DamageType Class Reference"))
  (returns (damageDealt :type Integer))
  (bind _returnvalue (- (stale _output_get) amount))
  (bind _output_get (set `self.currentHealth` _returnvalue))
  (set `self.combatTimer` 0)
  (return _returnvalue))

(fn `healActor`
  (params (amount :type Integer) (Source :type Byte))
  (bind _output_get (set `self.currentHealth` (+ (stale _output_get) amount)))
  (return))

(fn `regenHealth`
  (params (deltaSeconds :type "Float (double-precision)"))
  (locals (combatTimeout :type Integer :default 10))
  (bind _temphealth (`self.tempHealth`))
  (if (and (> (`self.combatTimer`) (`local.combatTimeout`)) (< (`self.percentHealth`) 1.0))
    (bind _output_get (set `self.tempHealth` (+ (stale _output_get) (* (`self.regenRate`) deltaSeconds))))
    (`|ExecutionSequence`
      (:`then_0`
        (if (>= _temphealth 1.0)
          (`/Engine/EditorBlueprintResources/StandardMacros.IncrementInt` (`self.currentHealth`)
            (:`  `
              (`/Engine/EditorBlueprintResources/StandardMacros.DecrementFloat` _temphealth)))))
      (:`then_1`
        (if (not (< (`self.percentHealth`) 1.0))
          (set `self.currentHealth` (`self.maxHealth`))))
      (:`then_2`
        (return)))
    (else
      (return))))

(fn `setupHealthSystem`
  (params (maxHealth :type Integer) (regenRate :type Integer))
  (bind _output_get (set `self.maxHealth` maxHealth))
  (set `self.currentHealth` _output_get)
  (set `self.regenRate` regenRate)
  (set `self.combatTimer` 1000000)
  (set `self.percentHealth` 1.0))

(fn `updateHealth`
  (params (`delta Seconds` :type "Float (double-precision)"))
  (`self.regenHealth` `delta Seconds`)
  (return))