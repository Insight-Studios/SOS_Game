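; Stamina component for a Character that manages sprinting, exhaustion and walk speed.
; Tick drains stamina while sprinting, by distance sprinted for BP_PlayerCharacter or by time for other owners.
; After sprinting stops, a retriggerable delay precedes regeneration.
; Sprinting doubles movement speed, while empty stamina causes exhaustion, halving speed and blocking sprint until stamina refills completely.
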(event `self.ReceiveBeginPlay`
  (`self.setupStaminaSystem` 1))

(event `self.ReceiveTick`
  (params (DeltaSeconds :type "Float (single-precision)"))
  (bind _ownermovementcomponent (`self.ownerMovementComponent`))
  (bind _normalwalkspeed (`self.normalWalkSpeed`))
  (`|ExecutionSequence`
    (:`then_0`
      (if (<= (`self.percentStamina`) 0.0)
        (set `self.exhausted` true)
        (`self.toggleSprint` false)))
    (:`then_1`
      (if (`self.isSprinting`)
        (bind _amount (`self.AmountToUse` DeltaSeconds))
        (`self.useStamina` _amount)
        (else
          (set `CharacterMovementComponent.MaxWalkSpeed` _normalwalkspeed _ownermovementcomponent)
          (if (`self.justUsed`)
            (set `self.justUsed` false)
            (`KismetSystemLibrary.RetriggerableDelay` 3.0)
            (set `self.regenning` true))
          (if (`self.regenning`)
            (`self.regenStamina` DeltaSeconds)))))
    (:`then_2`
      (if (`self.exhausted`)
        (set `CharacterMovementComponent.MaxWalkSpeed` (/ _normalwalkspeed 2.0) _ownermovementcomponent)))))

(fn `AmountToUse`
  (params (`Delta Seconds` :type "Float (double-precision)"))
  (returns (Amount :type "Float (double-precision)"))
  (locals (tempSprint :type "Float (double-precision)" :default 0.0))
  (bind _asbp_player_character (cast `/Game/Assets/Blueprints/Entities/Characters/Humans/BP_PlayerCharacter` (`self.GetOwner`))
    (:`then`
      (bind _totaldistancesprinted (`/Game/Assets/Blueprints/Entities/Characters/Humans/BP_PlayerCharacter.TotalDistanceSprinted` _asbp_player_character))
      (bind _output_get (set `local.tempSprint` (/ (- _totaldistancesprinted (`self.lastSprint`)) 100.0)))
      (set `self.lastSprint` _totaldistancesprinted)
      (return _output_get))
    (:`CastFailed`
      (return (* 10 `Delta Seconds`)))))

(fn `regenStamina`
  (params (`delta Seconds` :type "Float (double-precision)"))
  (bind _currentstamina (`self.currentStamina`))
  (bind _returnvalue (`KismetMathLibrary.Conv_IntToDouble` (`self.maxStamina`)))
  (if (< (`self.percentStamina`) 1.0)
    (set `self.currentStamina` (+ (* (`self.regenRate`) `delta Seconds`) _currentstamina))
    (else
      (set `self.currentStamina` _returnvalue)
      (set `self.exhausted` false)))
  (set `self.percentStamina` (/ _currentstamina _returnvalue)))

(fn `setupStaminaSystem`
  (params (`Max Stamina` :type Integer) (`regen Rate` :type Integer))
  (bind _output_get (set `self.maxStamina` `Max Stamina`))
  (set `self.currentStamina` (`KismetMathLibrary.Conv_IntToDouble` _output_get))
  (set `self.regenRate` `regen Rate`)
  (bind _ascharacter (cast `Character` (`self.GetOwner`)))
  (bind _charactermovement (`Character.CharacterMovement` _ascharacter))
  (set `self.normalWalkSpeed` (`CharacterMovementComponent.MaxWalkSpeed` _charactermovement))
  (set `self.ownerMovementComponent` _charactermovement))

(fn `toggleSprint`
  (params (sprinting :type Boolean))
  (bind _normalwalkspeed (`self.normalWalkSpeed`))
  (bind _ownermovementcomponent (`self.ownerMovementComponent`))
  (set `self.isSprinting` sprinting)
  (if (`self.exhausted`)
    (bind _output_get (set `self.isSprinting` false)))
  (if _output_get
    (set `CharacterMovementComponent.MaxWalkSpeed` (* _normalwalkspeed 2.0) _ownermovementcomponent)
    (else
      (set `CharacterMovementComponent.MaxWalkSpeed` _normalwalkspeed _ownermovementcomponent))))

(fn `useStamina`
  (params (amount :type "Float (double-precision)"))
  (returns (Used :type Boolean))
  (if (`self.exhausted`)
    (return false)
    (else
      (bind _output_get (set `self.currentStamina` (- (stale _output_get) amount)))
      (set `self.justUsed` true)
      (set `self.percentStamina` (/ (`self.currentStamina`) (`KismetMathLibrary.Conv_IntToDouble` (`self.maxStamina`))))
      (set `self.regenning` false)
      (return true))))