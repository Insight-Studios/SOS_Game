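; Sanguine Thirst skill that restores the player's water on kills.
; OnPurchase binds DrinkBlood to the player's kill-unit event, and MeetsConditions gates the skill through a prerequisite check.
; Each trigger adds level times kills over fifty times deaths to CurrentWater.
; That ratio is divided before float conversion and has no guard for zero deaths.
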(event `self.OnPurchase`
  (params (`Player Reference` :type "/Game/Assets/Blueprints/Entities/Characters/Humans/BP_PlayerCharacter Object Reference"))
  (add `/Game/Assets/Blueprints/Entities/Characters/BP_SOSCharacter.OnKillUnit` `Player Reference` (delegate `Drink Blood`)))

(event `Drink Blood`
  (set `/Game/Assets/Blueprints/Entities/Characters/Humans/BP_HumanCharacter.CurrentWater` (+ (`/Game/Assets/Blueprints/Entities/Characters/Humans/BP_HumanCharacter.CurrentWater` (stale `self.OnPurchase` `Player Reference`)) (* (`/Game/Assets/Blueprints/Entities/Characters/BP_SOSCharacter.CurrentLevel` (stale `self.OnPurchase` `Player Reference`)) (`KismetMathLibrary.Conv_IntToDouble` (/ (`/Game/Assets/Blueprints/Entities/Characters/Humans/BP_PlayerCharacter.KillCount` (stale `self.OnPurchase` `Player Reference`)) (* (`/Game/Assets/Blueprints/Entities/Characters/Humans/BP_PlayerCharacter.DeathCount` (stale `self.OnPurchase` `Player Reference`)) 50))))) (stale `self.OnPurchase` `Player Reference`)))

(fn `MeetsConditions`
  (params (`Player Reference` :type "/Game/Assets/Blueprints/Entities/Characters/Humans/BP_PlayerCharacter Object Reference"))
  (returns (`ConditionsMet?` :type Boolean))
  (bind _met_conditions (`self.CheckForPrerequisites` `Player Reference`))
  (return _met_conditions))