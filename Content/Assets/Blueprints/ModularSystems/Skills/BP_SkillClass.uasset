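; BP_SkillClass is a base skill class for a modular skill system, defining purchase and eligibility functions for a player.
; OnPurchase is an empty hook, and MeetsConditions returns true by default.
; CheckForPrerequisites counts exact class matches between PreRequisites and the player's AquiredSkills, passing when the count equals the number of prerequisites.
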(fn `CheckForPrerequisites`
  (params (`Player Reference` :type "/Game/Assets/Blueprints/Entities/Characters/Humans/BP_PlayerCharacter Object Reference"))
  (returns (`Met Conditions` :type Boolean))
  (locals (trueCount :type Integer))
  (bind _prerequisites (`self.PreRequisites`))
  (for _array_element _prerequisites
    (for _array_element_2 (`/Game/Assets/Blueprints/Entities/Characters/BP_SOSCharacter.AquiredSkills` `Player Reference`)
      (if (== _array_element (`GameplayStatics.GetObjectClass` _array_element_2))
        (bind _result (`/Engine/EditorBlueprintResources/StandardMacros.IncrementInt` (`local.trueCount`))))))
  (return (== _result (`KismetArrayLibrary.Array_Length` _prerequisites))))

(fn `MeetsConditions`
  (params (`Player Reference` :type "/Game/Assets/Blueprints/Entities/Characters/Humans/BP_PlayerCharacter Object Reference"))
  (returns (`ConditionsMet?` :type Boolean))
  (return true))

(fn `OnPurchase`
  (params (`Player Reference` :type "/Game/Assets/Blueprints/Entities/Characters/Humans/BP_PlayerCharacter Object Reference"))
  (return))