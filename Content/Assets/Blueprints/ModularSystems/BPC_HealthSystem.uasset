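; Health component that tracks an owner's current, max and percent health, with damage and out-of-combat regeneration.
; SetupHealthSystem sets the stats, and ApplyDamage subtracts health, resets the combat timer and prints the result.
; Tick regenerates health once the timer passes the timeout, capping at max, and calls OnDeath on a BP_Entity owner every frame health is at or below zero.
; ApplyHeal is an empty stub.
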(event `self.ReceiveBeginPlay`)

(event `self.ReceiveTick`
  (params (DeltaSeconds :type "Float (single-precision)"))
  (`|ExecutionSequence`
    (:`then_0`
      (`self.regenHealth` DeltaSeconds)
      (bind _output_get (set `self.combatTimer` (+ (stale _output_get) DeltaSeconds))))
    (:`then_1`
      (if (<= (`self.currentHealth`) 0.0)
        (bind _asbp_entity (cast `/Game/Assets/Blueprints/Entities/BP_Entity` (`self.GetOwner`)))
        (`/Game/Assets/Blueprints/Entities/BP_Entity.On Death` _asbp_entity)))))

(fn `applyDamage`
  (params (Damage :type "Float (double-precision)"))
  (bind _output_get (set `self.currentHealth` (- (stale _output_get) Damage)))
  (`self.updatePercent`
    (:`exec out`
      (set `self.combatTimer` 0.0)
      (`KismetSystemLibrary.PrintString` (`KismetStringLibrary.Concat_StrStr` (`KismetStringLibrary.Conv_DoubleToString` _output_get) " of " (`KismetStringLibrary.Conv_IntToString` (`self.maxHealth`)))))))

(fn `applyHeal`
  (params (Health :type "Float (double-precision)")))

(fn `regenHealth`
  (params (deltaSeconds :type "Float (double-precision)"))
  (if (and (> (`self.combatTimer`) (`self.combatTimeout`)) (< (`self.percentHealth`) 1.0))
    (`|ExecutionSequence`
      (:`then_0`
        (set `self.currentHealth` (+ (* (`self.regenRate`) deltaSeconds) (`self.currentHealth`)))
        (`self.updatePercent`))
      (:`then_1`
        (if (not (< (`self.percentHealth`) 1.0))
          (set `self.currentHealth` (`KismetMathLibrary.Conv_IntToDouble` (`self.maxHealth`)))
          (set `self.percentHealth` 1.0)))
      (:`then_2`
        (return)))))

(fn `setupHealthSystem`
  (params (maxHealth :type Integer) (regenRate :type Integer) (combatTimeout :type "Float (double-precision)"))
  (bind _output_get (set `self.maxHealth` maxHealth))
  (set `self.currentHealth` (`KismetMathLibrary.Conv_IntToDouble` _output_get))
  (set `self.regenRate` regenRate)
  (set `self.combatTimer` 1000000.0)
  (set `self.combatTimeout` combatTimeout)
  (set `self.percentHealth` 1.0))