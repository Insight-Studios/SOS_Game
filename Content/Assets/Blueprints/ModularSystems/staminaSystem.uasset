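; Stamina component for a Character owner that pairs a stamina pool with sprinting, which doubles the normal walk speed.
; Setup caches the movement component and base walk speed, while ToggleSprint switches between the two speeds.
; Tick forces sprint off at empty stamina, updates the stamina percentage, and drains stamina through a time-based accumulator, which is never reset.
; RegenStamina is called while not sprinting but is an empty stub.
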(event `self.ReceiveBeginPlay`
  (`self.setupStaminaSystem` 1))

(event `self.ReceiveTick`
  (params (DeltaSeconds :type "Float (single-precision)"))
  (`|ExecutionSequence`
    (:`then_0`
      (if (<= (`self.percentStamina`) 0.0)
        (`self.toggleSprint` false)))
    (:`then_1`
      (set `self.percentStamina` (/ (`KismetMathLibrary.Conv_IntToDouble` (`self.currentStamina`)) (`KismetMathLibrary.Conv_IntToDouble` (`self.maxStamina`)))))
    (:`then_2`
      (if (`self.isSprinting`)
        (bind _output_get (set `self.tempStamina` (+ (* 10 DeltaSeconds) (`self.tempStamina`))))
        (if (>= _output_get 1.0)
          (`self.useStamina` 1))
        (else
          (`self.regenStamina`))))))

(fn `regenStamina`)

(fn `setupStaminaSystem`
  (params (`Max Stamina` :type Integer))
  (bind _output_get (set `self.maxStamina` `Max Stamina`))
  (set `self.currentStamina` _output_get)
  (bind _ascharacter (cast `Character` (`self.GetOwner`)))
  (bind _charactermovement (`Character.CharacterMovement` _ascharacter))
  (set `self.normalWalkSpeed` (`CharacterMovementComponent.MaxWalkSpeed` _charactermovement))
  (set `self.ownerMovementComponent` _charactermovement))

(fn `toggleSprint`
  (params (sprinting :type Boolean))
  (bind _normalwalkspeed (`self.normalWalkSpeed`))
  (bind _ownermovementcomponent (`self.ownerMovementComponent`))
  (bind _output_get (set `self.isSprinting` sprinting))
  (if _output_get
    (set `CharacterMovementComponent.MaxWalkSpeed` (* _normalwalkspeed 2.0) _ownermovementcomponent)
    (else
      (set `CharacterMovementComponent.MaxWalkSpeed` _normalwalkspeed _ownermovementcomponent))))

(fn `useStamina`
  (params (amount :type Integer))
  (bind _output_get (set `self.currentStamina` (- (stale _output_get) amount))))