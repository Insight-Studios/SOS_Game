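; Spike hazard actor that repeatedly deals physical damage to the player while they overlap it.
; Begin and end overlap share logic that toggles a poking flag for the player pawn and primes the hit timer.
; While the flag is set, Tick damages the ThirdPersonCharacter's HealthSystem immediately, then about once per second.
; BeginPlay caches the GamayHUD, though the graph never uses it afterward.
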(event `self.ReceiveBeginPlay`
  (bind _asgamay_hud (cast `/Game/TopDownBP/Blueprints/GamayHUD` (`PlayerController.GetHUD` (`GameplayStatics.GetPlayerController` 0))))
  (set `self.GamayHUD` _asgamay_hud))

(event `self.ReceiveActorEndOverlap`
  (params (OtherActor :type "Actor Object Reference"))
  (if (== (stale `self.ReceiveActorBeginOverlap` OtherActor) (`GameplayStatics.GetPlayerPawn` 0)) :!label _label
    (set `self.pokingPlayer` (not (`self.pokingPlayer`)))
    (set `self.hitTime` 1.0)))

(event `self.ReceiveActorBeginOverlap`
  (params (OtherActor :type "Actor Object Reference"))
  (goto _label))

(event `self.ReceiveTick`
  (params (DeltaSeconds :type "Float (single-precision)"))
  (bind _hittime (`self.hitTime`))
  (if (`self.pokingPlayer`)
    (if (and (< (- _hittime DeltaSeconds) 1.0) (>= _hittime 1.0))
      (bind _asthird_person_character (cast `/Game/TopDownBP/Blueprints/ThirdPersonCharacter` (`GameplayStatics.GetPlayerPawn` 0)))
      (`/Game/Assets/Blueprints/ModularSystems/healthSystem.damageActor` (`/Game/TopDownBP/Blueprints/ThirdPersonCharacter.healthSystem` _asthird_person_character) 50 "/Game/Assets/Blueprints/DamageTypes/DamageType_Physical.DamageType_Physical_C")
      (set `self.hitTime` 0.0)
      (else
        (bind _output_get (set `self.hitTime` (+ (stale _output_get) DeltaSeconds)))))))

(fn `UserConstructionScript`)