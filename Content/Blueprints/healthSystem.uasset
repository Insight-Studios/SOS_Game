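; Health component that tracks an owning actor's current health, with functions to damage, heal and regenerate it.
; Tick runs a PerSecond macro that detects whole-second crossings in the owner's lifetime to apply regeneration about once a second.
; UpdateHealth also regenerates and computes the health percentage, but nothing in this file calls it.
; Health changes are unclamped, Source inputs are unused, and OnDeath is an empty stub.
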(event `self.ReceiveTick`
  (params (DeltaSeconds :type "Float (single-precision)"))
  (`self.perSecond` DeltaSeconds
    (:`PerSecond`
      (`self.regenHealth`))))

(fn `damageActor`
  (params (amount :type Integer) (Source :type "/Game/Blueprints/attributes Enum" :default "NewEnumerator0"))
  (bind _output_get (set `self.currentHealth` (- (stale _output_get) amount)))
  (return))

(fn `healActor`
  (params (amount :type Integer) (Source :type "/Game/Blueprints/attributes Enum" :default "NewEnumerator0"))
  (bind _output_get (set `self.currentHealth` (+ (stale _output_get) amount)))
  (return))

(fn `onDeath`)

(fn `regenHealth`
  (bind _output_get (set `self.currentHealth` (- (+ (stale _output_get) (`self.regenRate`)) (`self.-regen`))))
  (return))

(fn `updateHealth`
  (`self.regenHealth`)
  (set `self.percentHealth` (/ (`KismetMathLibrary.Conv_IntToDouble` (`self.currentHealth`)) (`KismetMathLibrary.Conv_IntToDouble` (`self.maxHealth`))))
  (return))