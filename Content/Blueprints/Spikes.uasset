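; Spikes is a hazard actor that damages the player's TopDownCharacter while the two overlap.
; Begin and end overlap share one branch that prints "Ouch" and toggles a PokingPlayer flag for the player pawn.
; Tick calls DamagePlayer with a fixed amount every frame while the flag is set, so damage depends on frame rate.
; BeginPlay caches the GamayHUD, which is otherwise unused here.
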(event `self.ReceiveBeginPlay`
  (bind _asgamay_hud (cast `/Game/TopDownBP/Blueprints/GamayHUD` (`PlayerController.GetHUD` (`GameplayStatics.GetPlayerController` 0))))
  (set `self.GamayHUD` _asgamay_hud))

(event `self.ReceiveActorEndOverlap`
  (params (OtherActor :type "Actor Object Reference"))
  (if (== (stale `self.ReceiveActorBeginOverlap` OtherActor) (`GameplayStatics.GetPlayerPawn` 0)) :!label _label
    (`KismetSystemLibrary.PrintString` "Ouch")
    (set `self.pokingPlayer` (not (`self.pokingPlayer`)))))

(event `self.ReceiveActorBeginOverlap`
  (params (OtherActor :type "Actor Object Reference"))
  (goto _label))

(event `self.ReceiveTick`
  (params (DeltaSeconds :type "Float (single-precision)"))
  (if (`self.pokingPlayer`)
    (bind _astop_down_character (cast `/Game/TopDownBP/Blueprints/TopDownCharacter` (`GameplayStatics.GetPlayerPawn` 0)))
    (`/Game/TopDownBP/Blueprints/TopDownCharacter.damagePlayer` _astop_down_character 2)))

(fn `UserConstructionScript`)